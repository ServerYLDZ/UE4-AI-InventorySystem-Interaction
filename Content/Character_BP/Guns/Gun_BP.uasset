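; Gun actor that serves as an interactable pickup and handles firing, ammo and a binocular aim view.
; Interacting drops the held item, shows the player's gun and ammo HUD, then destroys the pickup.
; Fire spawns a projectile per call, reloading from reserve when empty; HitScan adds a camera trace for decals and physics impulses, spending ammo only on hits.
; Binocular mode blends the view target to the gun and aims bullets along its Arrow.
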(event `/Game/Character_BP/İnteract_İnterface.LookAt`
  (params (PlayerCharac :type "/Game/Character_BP/Character_BP Object Reference"))
  (`/Game/Widgets/DisplayİtemWidget.UpdateDisplayMassage` (`/Game/Character_BP/Character_BP.Display HUD` PlayerCharac) "Press[E] To Take Hand"))

(event `/Game/Character_BP/İnteract_İnterface.İnteractWith`
  (params (PlayerChar :type "/Game/Character_BP/Character_BP Object Reference"))
  (bind _output_get (set `self.Player` PlayerChar))
  (bind _holdact (`/Game/Character_BP/Character_BP.HoldAct` _output_get)
    (:`then`
      (`/Game/İtem/Base_item.Drop` _holdact)
      (set `/Game/Character_BP/Character_BP.HoldAct` null _output_get))
    (:`else`
      _))
  (`self.TakeHand`)
  (set `/Game/Character_BP/Character_BP.hasRiffle` true _output_get)
  (set `/Game/Character_BP/Character_BP.GunisHand` true _output_get))

(event `/Game/Character_BP/İnteract_İnterface.Takeİnventer`
  (params (interacter :type "/Game/Character_BP/Character_BP Object Reference")))

(event `self.ReceiveTick`
  (params (DeltaSeconds :type "Float (single-precision)"))
  (if (`self.isBinoqculars`)
    (bind _ascharacter_bp (cast `/Game/Character_BP/Character_BP` (`GameplayStatics.GetPlayerCharacter` 0)))
    (`SceneComponent.K2_SetWorldRotation` (`/Game/Character_BP/Character_BP.Camera` _ascharacter_bp) (`Controller.GetControlRotation` (`GameplayStatics.GetPlayerController` 0)) false false)))

(event `StartFire`
  (set `self.isFire` true)
  (`self.Fire`))

(event `StopFire`
  (set `self.isFire` false))

(event `BinocularsStart`
  (set `self.isBinoqculars` true)
  (`PlayerController.SetViewTargetWithBlend` (`GameplayStatics.GetPlayerController` 0) self 0.3 "VTBlend_Linear" 0.0 false))

(event `BinocularStop`
  (set `self.isBinoqculars` false)
  (`PlayerController.SetViewTargetWithBlend` (`GameplayStatics.GetPlayerController` 0) (`self.GetParentActor`) 0.3 "VTBlend_Linear" 0.0 false))

(fn `Fire`
  (locals (Direction :type "Rotator Structure" :default (struct)))
  (if (`self.HitScan`)
    (bind _ascharacter_bp (cast `/Game/Character_BP/Character_BP` (`GameplayStatics.GetPlayerCharacter` 0)))
    (if (> (`self.AmmoCurrent`) 0)
      ;[1 1 1] spawn bullet
      (if (`self.isBinoqculars`)
        (set `local.Direction` (`SceneComponent.K2_GetComponentRotation` (`self.Arrow`)))
        (else
          (set `local.Direction` (`SceneComponent.K2_GetComponentRotation` (`/Game/Character_BP/Character_BP.Camera` _ascharacter_bp)))))
      (bind _returnvalue (`|SpawnActorFromClass` (`self.ProjectileBullet`) (`KismetMathLibrary.MakeTransform` (`SceneComponent.K2_GetComponentLocation` (`self.Scene`)) (`local.Direction`)) "Undefined" "OverrideRootScale" null null))
      (bind _projectilemovement (`/Game/Character_BP/Guns/Bullet.ProjectileMovement` _returnvalue))
      (set `ProjectileMovementComponent.InitialSpeed` (`self.BulletSpeed`) _projectilemovement)
      (set `ProjectileMovementComponent.MaxSpeed` (`self.BulletSpeed`) _projectilemovement)
      (bind _camera (`/Game/Character_BP/Character_BP.Camera` _ascharacter_bp))
      (bind _returnvalue_2 (`KismetMathLibrary.GetForwardVector` (`SceneComponent.K2_GetComponentRotation` _camera)))
      (set `self.GunLocation` _returnvalue_2)
      (bind _returnvalue_3 (`SceneComponent.K2_GetComponentLocation` _camera))
      (bind _outhit (`KismetSystemLibrary.LineTraceSingle` :`Start` _returnvalue_3 :`End` (+ (* _returnvalue_2 2000.0) _returnvalue_3) :`TraceChannel` "TraceTypeQuery1" :`bIgnoreSelf` false))
      (bind (_bblockinghit _binitialoverlap _time _distance _location _impactpoint _normal _impactnormal _physmat _hitactor _hitcomponent) (`GameplayStatics.BreakHitResult` _outhit))
      (`self.Hitimpact` _bblockinghit _hitcomponent _hitcomponent _impactpoint)
      (if _bblockinghit
        (bind _returnvalue_4 (`GameplayStatics.SpawnDecalAtLocation` "/Game/Character_BP/Guns/Bullet_Holle_Decal.Bullet_Holle_Decal" (5.0 5.0 5.0) _location (`KismetMathLibrary.MakeRotFromX` _normal)))
        (`SceneComponent.K2_AttachToComponent` _returnvalue_4 _hitcomponent "None" "KeepWorld" "KeepWorld" "KeepWorld" true)
        (`/Engine/EditorBlueprintResources/StandardMacros.DecrementInt` (`self.AmmoCurrent`)))
      (else
        (`self.Reload`)))
    (else
      (bind _ascharacter_bp_2 (cast `/Game/Character_BP/Character_BP` (`GameplayStatics.GetPlayerCharacter` 0)))
      (if (> (`self.AmmoCurrent`) 0)
        (if (`self.isBinoqculars`)
          (set `local.Direction` (`SceneComponent.K2_GetComponentRotation` (`self.Arrow`)))
          (else
            (set `local.Direction` (`SceneComponent.K2_GetComponentRotation` (`/Game/Character_BP/Character_BP.Camera` _ascharacter_bp_2)))))
        (bind _returnvalue_5 (`|SpawnActorFromClass` (`self.ProjectileBullet`) (`KismetMathLibrary.MakeTransform` (`SceneComponent.K2_GetComponentLocation` (`self.Scene`)) (`local.Direction`)) "Undefined" "OverrideRootScale" null null))
        (bind _projectilemovement_2 (`/Game/Character_BP/Guns/Bullet.ProjectileMovement` _returnvalue_5))
        (set `ProjectileMovementComponent.InitialSpeed` (`self.BulletSpeed`) _projectilemovement_2)
        (set `ProjectileMovementComponent.MaxSpeed` (`self.BulletSpeed`) _projectilemovement_2)
        (`/Engine/EditorBlueprintResources/StandardMacros.DecrementInt` (`self.AmmoCurrent`))
        (else
          (`self.Reload`))))))

(fn `Hitimpact`
  (params (isHittingSomething :type Boolean) (HitCommponent :type "SceneComponent Object Reference") (self3 :type "PrimitiveComponent Object Reference") (Location :type "Vector Structure"))
  (if isHittingSomething
    (if (`SceneComponent.IsSimulatingPhysics` HitCommponent "None")
      (`PrimitiveComponent.AddImpulseAtLocation` self3 (* (`self.GunLocation`) 200000.0) Location "None"))))

(fn `Reload`
  (locals (DiffiranceAmmo :type Integer))
  (bind _output_get (set `local.DiffiranceAmmo` (- (`self.ClipSize`) (`self.AmmoCurrent`))))
  (if (>= (`self.AmmoMax`) _output_get)
    (set `self.AmmoMax` (- (`self.AmmoMax`) _output_get))
    (set `self.AmmoCurrent` (+ (`self.AmmoCurrent`) (`local.DiffiranceAmmo`)))
    (else
      (set `self.AmmoCurrent` (+ (`self.AmmoCurrent`) (`self.AmmoMax`)))
      (set `self.AmmoMax` 0))))

(fn `TakeHand`
  (`SceneComponent.SetVisibility` (`/Game/Character_BP/Character_BP.Gun` (`self.Player`)) true false)
  (bind _asplayer_controller_bp (cast `/Game/Character_BP/PlayerController_BP` (`GameplayStatics.GetPlayerController` 0)))
  (`Widget.SetVisibility` (`/Game/Widgets/HUD.GunAmmo_2` (`/Game/Character_BP/PlayerController_BP.widgetHUD` _asplayer_controller_bp)) "Visible")
  (`self.K2_DestroyActor`))

(fn `UserConstructionScript`)