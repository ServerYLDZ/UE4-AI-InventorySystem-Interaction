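; M-16 gun Blueprint that provides automatic fire by overriding its parent's StartFire and StopFire events.
; StartFire calls the parent, copies FireRate1 into FireRate, fires immediately, then starts a looping timer that calls Fire by function name at that interval.
; StopFire calls the parent and clears the stored timer handle; Fire itself is not defined in these graphs.
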(event `self.StartFire`
  (`parent.StartFire`)
  (set `self.FireRate` (`self.FireRate_1`))
  (`self.Fire`)
  (bind _returnvalue (`KismetSystemLibrary.K2_SetTimer` null "Fire" (`self.FireRate`) true))
  (set `self.Timer` _returnvalue))

(event `self.StopFire`
  (`parent.StopFire`)
  (`KismetSystemLibrary.K2_ClearAndInvalidateTimerHandle` (`self.Timer`)))

(fn `UserConstructionScript`
  (`parent.UserConstructionScript`))