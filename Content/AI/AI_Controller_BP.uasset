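; AI controller that runs AI_BehaviorTree and feeds its blackboard from patrol settings and perception.
; On BeginPlay it copies the AI-1 pawn's patrol loop and wait time into blackboard keys.
; Perception updates treat stimulus index 0 as sight, setting CanSeePlayer, and index 1 as hearing, storing its location and always flagging it heard.
; Older tag-based perception and obstacle-jump logic remain unconnected.
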(event `self.ReceiveBeginPlay`
  (bind _returnvalue (`AIBlueprintHelperLibrary.GetBlackboard` null))
  (`self.RunBehaviorTree` "/Game/AI/AI_BehaviorTree.AI_BehaviorTree")
  (bind _asai_1 (cast `/Game/AI/AI-1` (`self.K2_GetPawn`)))
  (`BlackboardComponent.SetValueAsBool` _returnvalue "isLoop" (`/Game/AI/PatrolPoint.isLoop` (`/Game/AI/AI-1.Patrol` _asai_1)))
  (`BlackboardComponent.SetValueAsBool` _returnvalue "ReverseLooPath" false)
  (`BlackboardComponent.SetValueAsFloat` _returnvalue "WaitTime" (`/Game/AI/PatrolPoint.WaitTime` (`/Game/AI/AI-1.Patrol` _asai_1))))

(event `self.AIPerception.OnTargetPerceptionUpdated`
  (params (Actor :type "Actor Object Reference") (Stimulus :type "AIStimulus Structure"))
  ;[1 1 1] silinebilir
)

(event `self.AIPerception.OnPerceptionUpdated`
  (params (UpdatedActors :type "Array of Actor Object Reference (by ref)"))
  (for _array_element UpdatedActors
    (bind _info (`AIPerceptionComponent.GetActorsPerception` (`self.AIPerception`) _array_element))
    (`self.Perception` (`.LastSensedStimuli` (break `ActorPerceptionBlueprintInfo` _info)))))

(event `self.ReceivePossess`
  (params (PossessedPawn :type "Pawn Object Reference"))
  (bind _ascharacter (cast `Character` PossessedPawn))
  (set `self.PawnAI` _ascharacter))

(event `self.ReceiveTick`
  (params (DeltaSeconds :type "Float (single-precision)")))

(fn `Perception`
  (params (Array :type "Array of AIStimulus Structure"))
  (locals (Percceptions :type "AIStimulus Structure"))
  (for (_array_element _array_index) Array
    (bind _output_get (set `local.Percceptions` _array_element))
    (switch `int` _array_index
      (:`0`
        (bind (_age _expirationage _strength _stimuluslocation _receiverlocation _tag _bsuccessfullysensed) (break `AIStimulus` _output_get))
        (`BlackboardComponent.SetValueAsBool` (`AIBlueprintHelperLibrary.GetBlackboard` null) "CanSeePlayer" _bsuccessfullysensed))
      (:`1`
        (`BlackboardComponent.SetValueAsBool` (`AIBlueprintHelperLibrary.GetBlackboard` null) "isHearingSameThing" true)
        (`BlackboardComponent.SetValueAsVector` (`AIBlueprintHelperLibrary.GetBlackboard` null) "RandomLocTarget" _stimuluslocation)))))

(fn `UserConstructionScript`)